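; BP_Controller is a controller Blueprint that owns the on-screen health and score UI.
; On BeginPlay it creates the Health_UI and Score_UI widgets, stores references to them and adds both to the viewport.
; Its UpdateHealthbar and UpdateScore events pass incoming values straight to those widgets, so the controller acts as a relay between game state and HUD.
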(event `UpdateScore`
  (params (CurrentScore :type Integer))
  (`/Game/InfiniteMatrix/UI/Score_UI.SetScoreInfo` (`self.Score_UI`) CurrentScore))

(event `UpdateHealthbar`
  (params (Currenthealth :type "Float (double-precision)") (Maxhealth :type "Float (double-precision)"))
  (`/Game/InfiniteMatrix/UI/Health_UI.SetHealthBarInfo` (`self.Health_UI`) Currenthealth Maxhealth))

(event `self.ReceiveBeginPlay`
  (bind _returnvalue (`|CreateWidget` "/Game/InfiniteMatrix/UI/Health_UI.Health_UI_C"))
  (bind _output_get (set `self.Health_UI` _returnvalue))
  (`UserWidget.AddToViewport` _output_get 0)
  (bind _returnvalue_2 (`|CreateWidget` "/Game/InfiniteMatrix/UI/Score_UI.Score_UI_C"))
  (bind _output_get_2 (set `self.Score_UI` _returnvalue_2))
  (`UserWidget.AddToViewport` _output_get_2 0))

(fn `UserConstructionScript`)